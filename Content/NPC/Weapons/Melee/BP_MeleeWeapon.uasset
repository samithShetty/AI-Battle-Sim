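; BP_MeleeWeapon is a melee weapon actor that damages NPCs of an opposing team on overlap.
; On BeginPlay it casts its parent actor to BP_NPC_Base and stores it as the Wielder.
; HandleHit compares the overlapped NPC's Team to the Wielder's and applies WeaponDamage with the Wielder as causer.
; An EnemiesHit list stops repeat damage to the same NPC, and nothing in this Blueprint clears it.
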(event `self.ReceiveBeginPlay`
  (bind _asbp_npc_base (cast `/Game/NPC/Classes/BP_NPC_Base` (`self.GetParentActor`)))
  (set `self.wielder` _asbp_npc_base))

(event `self.ReceiveActorBeginOverlap`
  (params (OtherActor :type "Actor Object Reference"))
  (`self.HandleHit` OtherActor))

(fn `HandleHit`
  (params (`Hit Actor` :type "Actor Object Reference"))
  (bind _enemieshit (`self.enemiesHit`))
  (bind _asbp_npc_base (cast `/Game/NPC/Classes/BP_NPC_Base` `Hit Actor`))
  (if (!= (`/Game/NPC/Classes/BP_NPC_Base.team` _asbp_npc_base) (`/Game/NPC/Classes/BP_NPC_Base.team` (`self.wielder`)))
    (if (not (`BlueprintSetLibrary.Set_Contains` _enemieshit _asbp_npc_base))
      (`BlueprintSetLibrary.Set_Add` _enemieshit _asbp_npc_base)
      (`GameplayStatics.ApplyDamage` _asbp_npc_base (`self.weaponDamage`) null (`self.wielder`)))))

(fn `UserConstructionScript`)