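; BP_NPC_Spawner is a damageable, team-owned NPC spawner that is captured instead of destroyed when it dies.
; AnyDamage records the attacking NPC's team before passing damage to the parent, and ignores damage from non-BP_NPC_Base causers.
; On Die, it switches to the last attacker's team, recolors, restores full health and calls SpawnerCaptured, updating team population before and after the switch.
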(event `self.Die`
  (`self.Update Team Population` false)
  (set `self.team` (`self.attackerTeam`))
  (`self.Assign Team Color`)
  (set `self.Health` (`self.maxHealth`))
  (`self.SpawnerCaptured` self)
  (`self.Update Team Population` true))

(event `self.ReceiveAnyDamage`
  (params (Damage :type "Float (single-precision)") (DamageType :type "DamageType Object Reference") (InstigatedBy :type "Controller Object Reference") (DamageCauser :type "Actor Object Reference"))
  (bind _asbp_npc_base (cast `/Game/NPC/Classes/BP_NPC_Base` DamageCauser))
  (set `self.attackerTeam` (`/Game/NPC/Classes/BP_NPC_Base.team` _asbp_npc_base))
  (`parent.ReceiveAnyDamage` Damage null null null))

(fn `UserConstructionScript`
  (`parent.UserConstructionScript`))