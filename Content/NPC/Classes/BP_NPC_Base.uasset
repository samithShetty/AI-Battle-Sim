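; Base NPC character for a team battle simulation, with health, melee attacks, team body color and a health bar widget.
; Construction applies team color and stats, while spawn and death update team and total populations in BP_GameMode_BattleSim.
; Damage plays a hit montage or triggers Die, which detaches the controller and destroys the actor after its death montage.
; Attack enables weapon collision, EndAttack disables it and clears hit enemies, and Block is a stub.
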(event `self.ReceiveBeginPlay`
  (`self.Update Team Population` true)
  (bind _returnvalue (`|CreateWidget` "/Game/NPC/Extra/W_HealthBar.W_HealthBar_C" null self))
  (`WidgetComponent.SetWidget` (`self.HealthBar`) _returnvalue))

(event `self.ReceiveAnyDamage`
  (params (Damage :type "Float (single-precision)") (DamageType :type "DamageType Object Reference") (InstigatedBy :type "Controller Object Reference") (DamageCauser :type "Actor Object Reference"))
  (bind _hitstun (`self.Take Damage` Damage))
  (`KismetSystemLibrary.Delay` _hitstun))

(event `Die`
  (`self.DetachFromControllerPendingDestroy`)
  (set `PrimitiveComponent.bGenerateOverlapEvents` false (`self.CapsuleComponent`))
  (`self.Update Team Population` false)
  (bind _returnvalue (`self.PlayAnimMontage` "/Game/Assets/Characters/Mannequin_UE4/Animations/Montage_Death.Montage_Death"))
  (`KismetSystemLibrary.Delay` _returnvalue)
  (`self.K2_DestroyActor`))

(event `/Game/NPC/AI/BP_AI_BehaviorTrees.EndAttack`
  (bind _asbp_melee_weapon (cast `/Game/NPC/Weapons/Melee/BP_MeleeWeapon` (`ChildActorComponent.ChildActor` (`self.Weapon`)) :!pure true))
  (`BlueprintSetLibrary.Set_Clear` (`/Game/NPC/Weapons/Melee/BP_MeleeWeapon.enemiesHit` _asbp_melee_weapon))
  (`PrimitiveComponent.SetCollisionEnabled` (`/Game/NPC/Weapons/Melee/BP_MeleeWeapon.StaticMesh` _asbp_melee_weapon) "NoCollision"))

(fn `Assign Team Color`
  (bind _team (`self.team`)
    (:`then`
      (bind _returnvalue (`PrimitiveComponent.CreateDynamicMaterialInstance` (`self.Mesh`) 0 "/Game/Assets/Characters/Mannequin_UE4/Materials/M_MannequinUE4_Body.M_MannequinUE4_Body" "None"))
      (`MaterialInstanceDynamic.SetVectorParameterValue` _returnvalue "BodyColor" (`KismetMathLibrary.Conv_ColorToLinearColor` (`/Game/Teams/TeamDataAsset.TeamColor` _team))))
    (:`else`)))

(fn `Attack`
  (returns (animationDuration :type "Float (double-precision)"))
  (bind _returnvalue (`self.PlayAnimMontage` "/Game/Assets/Characters/Mannequin_UE4/Animations/Montage_Punch.Montage_Punch"))
  (bind _asbp_melee_weapon (cast `/Game/NPC/Weapons/Melee/BP_MeleeWeapon` (`ChildActorComponent.ChildActor` (`self.Weapon`))))
  (`PrimitiveComponent.SetCollisionEnabled` (`/Game/NPC/Weapons/Melee/BP_MeleeWeapon.StaticMesh` _asbp_melee_weapon) "QueryAndPhysics")
  (return _returnvalue))

(fn `Block`
  (returns (animationDuration :type "Float (double-precision)"))
  (return 0.0))

(fn `Take Damage`
  (params (damage :type "Float (double-precision)"))
  (returns (hitStun :type "Float (double-precision)"))
  (bind _output_get (set `self.Health` (- (`self.Health`) damage)))
  (if (<= _output_get 0.0)
    (`self.Die`)
    (else
      (bind _returnvalue (`self.PlayAnimMontage` "/Game/Assets/Characters/Mannequin_UE4/Animations/Montage_Hit.Montage_Hit"))
      (return _returnvalue))))

(fn `Update Team Population`
  (params (`Plus/Minus` :type Boolean))
  (bind _returnvalue (`KismetMathLibrary.SelectInt` 1 -1 `Plus/Minus`))
  (bind _team (`self.team`))
  (bind _asbp_game_mode_battle_sim (cast `/Game/ThirdPerson/Blueprints/BP_GameMode_BattleSim` (`GameplayStatics.GetGameMode`)))
  (bind _team_populations (`/Game/ThirdPerson/Blueprints/BP_GameMode_BattleSim.Team Populations` _asbp_game_mode_battle_sim))
  (`BlueprintMapLibrary.Map_Add` _team_populations _team (+ (`BlueprintMapLibrary.Map_Find` _team_populations _team) _returnvalue))
  (set `/Game/ThirdPerson/Blueprints/BP_GameMode_BattleSim.Total Population` (+ (`/Game/ThirdPerson/Blueprints/BP_GameMode_BattleSim.Total Population` _asbp_game_mode_battle_sim) _returnvalue) _asbp_game_mode_battle_sim))

(fn `UserConstructionScript`
  (`self.Assign Team Color`)
  ;[1 1 1] Set Character Stats
  (set `self.Health` (`self.maxHealth`))
  (set `CharacterMovementComponent.MaxWalkSpeed` (`self.moveSpeed`) (`self.CharacterMovement`)))