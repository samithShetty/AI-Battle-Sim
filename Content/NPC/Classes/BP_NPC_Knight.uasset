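; Knight NPC child Blueprint that fights with a sword swing and a shield block, extending its parent NPC behavior.
; Attack plays the swing montage and enables query collision on the child-actor melee weapon; EndAttack disables it and clears the weapon's hit-enemy list.
; Block plays the shield montage and sets IsBlocking, which makes AnyDamage skip the parent's damage handling entirely until EndBlock clears the flag.
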(event `self.ReceiveBeginPlay`
  (`parent.ReceiveBeginPlay`))

(event `/Game/NPC/AI/BP_AI_BehaviorTrees.EndAttack`
  (bind _asbp_melee_weapon (cast `/Game/NPC/Weapons/Melee/BP_MeleeWeapon` (`ChildActorComponent.ChildActor` (`self.Weapon`)) :!pure true))
  (`BlueprintSetLibrary.Set_Clear` (`/Game/NPC/Weapons/Melee/BP_MeleeWeapon.enemiesHit` _asbp_melee_weapon))
  (`PrimitiveComponent.SetCollisionEnabled` (`/Game/NPC/Weapons/Melee/BP_MeleeWeapon.StaticMesh` _asbp_melee_weapon) "NoCollision"))

(event `self.ReceiveAnyDamage`
  (params (Damage :type "Float (single-precision)") (DamageType :type "DamageType Object Reference") (InstigatedBy :type "Controller Object Reference") (DamageCauser :type "Actor Object Reference"))
  (if (not (`self.isBlocking`))
    (`parent.ReceiveAnyDamage` Damage DamageType InstigatedBy DamageCauser)))

(event `/Game/NPC/AI/BP_AI_BehaviorTrees.EndBlock`
  (set `self.isBlocking` false))

(fn `Attack`
  (returns (animationDuration :type "Float (double-precision)"))
  (bind _returnvalue (`self.PlayAnimMontage` "/Game/Assets/Characters/Mannequin_UE4/Animations/Montage_Sword_Swing.Montage_Sword_Swing"))
  (bind _asbp_melee_weapon (cast `/Game/NPC/Weapons/Melee/BP_MeleeWeapon` (`ChildActorComponent.ChildActor` (`self.Weapon`))))
  (`PrimitiveComponent.SetCollisionEnabled` (`/Game/NPC/Weapons/Melee/BP_MeleeWeapon.StaticMesh` _asbp_melee_weapon) "QueryOnly")
  (return _returnvalue))

(fn `Block`
  (returns (animationDuration :type "Float (double-precision)"))
  (set `self.isBlocking` true)
  (bind _returnvalue (`self.PlayAnimMontage` "/Game/Assets/Characters/Mannequin_UE4/Animations/Montage_Shield_Block.Montage_Shield_Block"))
  (return _returnvalue))

(fn `UserConstructionScript`
  (`parent.UserConstructionScript`))